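; Game mode for the Metaverse multiplayer game that tracks connected player controllers and handles spawning and kicking.
; Login triggers client spawning, and both login and logout update the controller list, then refresh player-list widgets locally after a short delay.
; SpawnPlayer replaces any existing pawn with the character class stored in the game instance, at a random PlayerStart.
; KickPlayer removes players by list index through their controller's owning-client kick call.
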(event Custom|UpdatePlayerList
  ;[1 1 1] Update Player List (Game Mode)
  (Utilities|FlowControl|Delay 0.2)
  (bind _foundwidgets (Widget|GetAllWidgetsOfClass "/Game/Network/Widget/WBP_PlayerList.WBP_PlayerList_C" false))
  (for _array_element _foundwidgets
    (Default|UpdateWidget _array_element)))

(event EventPostLogin
  (params (NewPlayer :type Player%20Controller%20Object%20Reference))
  ;[1 1 1] When a player is connected (Must check all players)
  (bind _aspc_metaverse (Utilities|Casting|CastToPC_Metaverse NewPlayer))
  (Utilities|FlowControl|Sequence
    (:then_0
      (Default|ClientSpawnPlayer _aspc_metaverse))
    (:then_1
      (Utilities|Array|Add (Variables|Default|GetAllPlayersController) _aspc_metaverse)
      ;[1 1 1] Access to Update Player List
      (CallFunction|UpdatePlayerList))))

(event EventOnSwapPlayerControllers
  (params (OldPC :type Player%20Controller%20Object%20Reference) (NewPC :type Player%20Controller%20Object%20Reference))
  ;[1 1 1] When a player is connected (Must check all players)
  (Utilities|Array|Add (Variables|Default|GetJoinPlayers) NewPC))

(event EventOnLogout
  (params (ExitingController :type Controller%20Object%20Reference))
  ;[1 1 1] When a player is disconnected
  (bind _aspc_metaverse (Utilities|Casting|CastToPC_Metaverse ExitingController))
  (Utilities|Array|RemoveItem (Variables|Default|GetAllPlayersController) _aspc_metaverse)
  ;[1 1 1] Access to Update Player List
  (CallFunction|UpdatePlayerList))

(fn ConstructionScript)

(fn FindRandomPlayerStart
  (bind _outactors (Actor|GetAllActorsOfClass "/Script/Engine.PlayerStart"))
  (return (Transformation|GetActorTransform (Utilities|Array|Get(acopy) _outactors (Math|Random|RandomIntegerinRange 0 (- (Utilities|Array|Length _outactors) 1))))))

(fn SpawnPlayer
  (params (PlayerController :type Player%20Controller%20Object%20Reference))
  (bind _returnvalue (Pawn|GetControlledPawn PlayerController))
  (Utilities|IsValid _returnvalue
    (:Is%20Valid
      (Actor|DestroyActor _returnvalue))
    (:Is%20Not%20Valid
      _))
  (bind _returnvalue_2 (Game|SpawnActorfromClass (Variables|/Game/Network/Core/GI_Metaverse.GI_Metaverse_C|GetCharacter (.AsGI%20Metaverse (Utilities|Casting|CastToGI_Metaverse (Game|GetGameInstance)))) (Spawning(ReferenceUsed)|FindRandomPlayerStart) "Undefined" 0 0))
  (Pawn|Possess PlayerController _returnvalue_2))

(fn KickPlayer
  (params (PlayerID :type Integer))
  (Default|OwingClientKickPlayer (Utilities|Array|Get(acopy) (Variables|Default|GetAllPlayersController) PlayerID)))